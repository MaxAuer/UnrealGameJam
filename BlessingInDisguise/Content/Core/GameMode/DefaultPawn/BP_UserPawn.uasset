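; BP_UserPawn is a pawn that smoothly follows a Target actor along the world X axis.
; Each Tick it caches the Target's X location, then uses FInterpTo with delta time and FollowSpeed to ease its own X toward that value.
; Its Y and Z stay unchanged, so the follow is locked to a single axis.
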(event `self.ReceiveActorBeginOverlap`
  (params (OtherActor :type "Actor Object Reference")))

(event `self.ReceiveTick`
  (params (DeltaSeconds :type "Float (single-precision)"))
  (`self.setTargetX`)
  (`self.smoothFollow` DeltaSeconds))

(fn `setTargetX`
  (bind _returnvalue_x (`KismetMathLibrary.BreakVector` (`self.K2_GetActorLocation` (`self.Target`))))
  (set `self.targetX` _returnvalue_x))

(fn `smoothFollow`
  (params (A :type "Float (double-precision)"))
  (bind (_returnvalue_x _returnvalue_y _returnvalue_z) (`KismetMathLibrary.BreakVector` (`self.K2_GetActorLocation`)))
  (bind _returnvalue_x_2 (`KismetMathLibrary.BreakVector` (`self.K2_GetActorLocation`)))
  (`self.K2_SetActorLocation` (`KismetMathLibrary.MakeVector` (`KismetMathLibrary.FInterpTo` _returnvalue_x_2 (`self.targetX`) A (`self.followSpeed`)) _returnvalue_y _returnvalue_z)))

(fn `UserConstructionScript`)