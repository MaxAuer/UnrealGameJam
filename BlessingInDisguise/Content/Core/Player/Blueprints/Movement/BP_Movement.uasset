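; BP_Movement is a player movement component that drives its owning actor forward along world +X with automatic acceleration.
; Each tick it updates a clamped speed from acceleration over delta time, minus any deceleration from DecelerateCharacter, which applies once and then resets.
; The next location is the current one offset by speed, smoothed with VInterpTo and set without sweeping.
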(event `self.ReceiveBeginPlay`
  (`self.setActor`)
  (`self.setStartPosition`))

(event `self.ReceiveTick`
  (params (DeltaSeconds :type "Float (single-precision)"))
  (`self.calculateCurrentSpeed`)
  (bind _newposition (`self.calculateNextPosition` (`self.StartLocation`) (`self.currentSpeed`) (1.0 0.0 0.0)))
  (`Actor.K2_SetActorLocation` (`self.Actor`) _newposition false false)
  (`self.setStartPosition`))

(fn `calculateCurrentSpeed`
  (set `self.currentSpeed` (`KismetMathLibrary.FClamp` (- (+ (`self.currentSpeed`) (* (`GameplayStatics.GetWorldDeltaSeconds`) (`self.acceleration`))) (`self.deceleration`)) 0.0 (`self.maxSpeed`)))
  (set `self.deceleration` 0.0))

(fn `calculateNextPosition`
  (params (currentPosition :type "Vector Structure") (Speed :type "Float (double-precision)") (Forward :type "Vector Structure"))
  (returns (newPosition :type "Vector Structure"))
  (return (`KismetMathLibrary.VInterpTo` currentPosition (+ currentPosition (* Forward Speed)) (`GameplayStatics.GetWorldDeltaSeconds`) 150.0)))

(fn `decelerateCharacter`
  (params (amount :type "Float (double-precision)"))
  (returns (return :type Boolean))
  (set `self.deceleration` amount)
  (return false))

(fn `setActor`
  (set `self.Actor` (`self.GetOwner`)))

(fn `setStartPosition`
  (set `self.StartLocation` (`Actor.K2_GetActorLocation` (`self.Actor`))))