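; A logic tile actor that sends a car component moving when a BP_Character overlaps it.
; The overlap sets a start flag, and Tick then advances an alpha by delta time times speed, lerping the car's relative location from a start to a target position.
; When the alpha would pass the end, the car component is destroyed.
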(event `self.ReceiveActorBeginOverlap`
  (params (OtherActor :type "Actor Object Reference"))
  (cast `/Game/Core/Player/Blueprints/BP_Character` OtherActor)
  (set `self.start` true))

(event `self.ReceiveTick`
  (params (DeltaSeconds :type "Float (single-precision)"))
  (bind _bid_car_v02_00 (`self.BID_Car_v02-00`))
  (bind _returnvalue (+ (`self.currentLerp`) (* DeltaSeconds (`self.speed`))))
  (if (`self.start`)
    (`/Engine/EditorBlueprintResources/StandardMacros.IsValid` (`self.BID_Car_v02-00`)
      (:`Is Valid`
        (if (> _returnvalue 1.0)
          (`ActorComponent.K2_DestroyComponent` _bid_car_v02_00)
          (else
            (set `self.currentLerp` _returnvalue)
            (`SceneComponent.K2_SetRelativeLocation` _bid_car_v02_00 (`KismetMathLibrary.VLerp` (`self.startPos`) (`self.targetPos`) (`self.currentLerp`)) false false)))))))

(fn `UserConstructionScript`)