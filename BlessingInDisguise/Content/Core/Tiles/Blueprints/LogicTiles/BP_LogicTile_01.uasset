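; BP_LogicTile_01 is a logic tile with a piano trap that is triggered when BP_Character overlaps it.
; The overlap sets a Start flag, and Tick then turns on physics simulation for the piano.
; A gated one-second delay afterwards disables the collider on the BP_Killable child actor and closes the gate.
; Randomized smash playback on piano overlap exists but is unconnected and never runs.
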(event `self.ReceiveActorBeginOverlap`
  (params (OtherActor :type "Actor Object Reference"))
  (cast `/Game/Core/Player/Blueprints/BP_Character` OtherActor)
  (set `self.start` true))

(event `self.ReceiveTick`
  (params (DeltaSeconds :type "Float (single-precision)"))
  (if (`self.start`)
    (`|ExecutionSequence`
      (:`then_0`
        (`KismetSystemLibrary.Delay` 0.0)
        (`PrimitiveComponent.SetSimulatePhysics` (`self.BID_Piano_v01-00`) true))
      (:`then_1`
        (`/Engine/EditorBlueprintResources/StandardMacros.Gate` false :!label _label
          (:`Exit`
            (`KismetSystemLibrary.Delay` 1.0)
            (bind _asbp_killable (cast `/Game/Core/Gameplay/BP_Killable` (`ChildActorComponent.ChildActor` (`self.BP_Killable`))))
            (`/Game/Core/Gameplay/BP_Killable.disableCollider` _asbp_killable)
            (goto _label :!via `Close`)))))))

(fn `UserConstructionScript`)