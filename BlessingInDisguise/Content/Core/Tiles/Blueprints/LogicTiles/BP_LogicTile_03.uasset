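; BP_LogicTile_03 is a logic tile that animates a grandma component when a BP_Character overlaps it.
; BeginPlay caches the component's relative start position and a target offset along local Y.
; After a short delay following the overlap, a flag lets Tick lerp the component toward the target by a Speed-scaled alpha.
; The component is destroyed once the next step would pass the end of the lerp.
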(event `self.ReceiveBeginPlay`
  (set `self.startPos` (`SceneComponent.RelativeLocation` (`self.BP_Grandma`)))
  (set `self.targetPos` (+ (`self.startPos`) (0.0 300.0 0.0))))

(event `self.ReceiveActorBeginOverlap`
  (params (OtherActor :type "Actor Object Reference"))
  (cast `/Game/Core/Player/Blueprints/BP_Character` OtherActor)
  (`KismetSystemLibrary.Delay` 1.75)
  (set `self.start` true))

(event `self.ReceiveTick`
  (params (DeltaSeconds :type "Float (single-precision)"))
  (bind _bp_grandma (`self.BP_Grandma`))
  (bind _returnvalue (+ (`self.currentLerp`) (* DeltaSeconds (`self.speed`))))
  (if (`self.start`)
    (`/Engine/EditorBlueprintResources/StandardMacros.IsValid` (`self.BP_Grandma`)
      (:`Is Valid`
        (if (> _returnvalue 1.0)
          (`ActorComponent.K2_DestroyComponent` _bp_grandma)
          (else
            (set `self.currentLerp` _returnvalue)
            (`SceneComponent.K2_SetRelativeLocation` _bp_grandma (`KismetMathLibrary.VLerp` (`self.startPos`) (`self.targetPos`) (`self.currentLerp`)) false false)))))))

(fn `UserConstructionScript`)