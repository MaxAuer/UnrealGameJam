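; BP_LogicTile_04 is a logic tile that links a child manhole actor to a killable component.
; On BeginPlay it binds the manhole's click event, whose handler destroys the BPKillable component.
; A BP_Character overlap sets a start flag after a short delay, letting Tick advance a clamped lerp alpha.
; The SetRelativeLocation lerp and a second DestroyComponent are unwired, so that alpha moves nothing.
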(event `test`
  (`ActorComponent.K2_DestroyComponent` (`self.BP_Killable`)))

(event `self.ReceiveBeginPlay`
  (bind _asbp_manhole (cast `/Game/Gameplay/Decelerator/BP_Manhole` (`ChildActorComponent.ChildActor` (`self.BP_Manhole`))))
  (add `/Game/Core/Gameplay/BP_Clickable.eventOnClick` _asbp_manhole (delegate `test`)))

(event `self.ReceiveActorBeginOverlap`
  (params (OtherActor :type "Actor Object Reference"))
  (cast `/Game/Core/Player/Blueprints/BP_Character` OtherActor)
  (`KismetSystemLibrary.Delay` 1.75)
  (set `self.start` true))

(event `self.ReceiveTick`
  (params (DeltaSeconds :type "Float (single-precision)"))
  (bind _returnvalue (+ (`self.currentLerp`) (* DeltaSeconds (`self.speed`))))
  (if (`self.start`)
    (`/Engine/EditorBlueprintResources/StandardMacros.IsValid` null
      (:`Is Valid`
        (if (not (> _returnvalue 1.0))
          (set `self.currentLerp` _returnvalue))))))

(fn `UserConstructionScript`)