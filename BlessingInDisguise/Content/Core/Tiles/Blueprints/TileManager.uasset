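; TileManager streams random tile actors along the X axis ahead of BP_Character, forming an endless track.
; BeginPlay finds the character and spawns a starting row of tiles offset from its position, beginning behind it.
; Each Tick compares the character's X to a threshold derived from tile count, size and look-ahead.
; Crossing it spawns a tile at the front and destroys the oldest, keeping a rolling window in ActiveActorArray.
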(event `self.ReceiveBeginPlay`
  (`self.GetCharacter`) ; Get the player character \nat game start
  ;[1 1 1] Loop over maximum number of tiles and create the starting scene.
  (for _index (range (+ (`self.MaxTiles`) 1))
    (set `self.TileCount` _index)
    (bind _tileactor (`self.GetRandomTile` (`self.TileActorArray`)))
    (`self.SpawnTileAtStart` _tileactor)))

(event `self.ReceiveTick`
  (params (DeltaSeconds :type "Float (single-precision)"))
  (bind (_newtileneeded _spawnposition) (`self.NeedNewTile`)) ; Check the position of the player and \ndecided whether or not to spawn a \nnew tile.
  (if _newtileneeded
    (bind _tileactor (`self.GetRandomTile` (`self.TileActorArray`)))
    (`self.SpawnTile` _tileactor _tileactor _spawnposition)))

(fn `GetCharacter`
  (bind _outactors (`GameplayStatics.GetAllActorsOfClass` "/Game/Core/Player/Blueprints/BP_Character.BP_Character_C"))
  (set `self.Character` (`|GetArrayItem` _outactors)))

(fn `GetRandomTile`
  (params (TileActorArray :type "Array of Actor Class Reference"))
  (returns (TileActor :type "Actor Class Reference"))
  (return (`|GetArrayItem` TileActorArray (`KismetMathLibrary.RandomIntegerInRange` 0 (- (`KismetArrayLibrary.Array_Length` TileActorArray) 1)))))

(fn `NeedNewTile`
  (returns (newTileNeeded :type Boolean) (SpawnPosition :type "Vector Structure"))
  (bind _tilesize (`self.TileSize`))
  (bind _returnvalue (* _tilesize (`self.TilesInAdvance`)))
  (bind _returnvalue_2 (`KismetMathLibrary.Conv_IntToDouble` (- (* (- (`self.TileCount`) 1) _tilesize) _returnvalue)))
  (return (>= (.x (`Actor.K2_GetActorLocation` (`self.Character`))) _returnvalue_2) (`KismetMathLibrary.MakeVector` (+ _returnvalue_2 (`KismetMathLibrary.Conv_IntToDouble` _returnvalue)) (+ (.y (`Actor.K2_GetActorLocation` (`self.Character`))) (`self.TileY`)))))

(fn `SpawnTile`
  (params (Class :type "Actor Class Reference") (NewItem :type "Actor Class Reference (by ref)") (Location :type "Vector Structure"))
  (bind _activeactorarray (`self.ActiveActorArray`))
  (bind _returnvalue (`|SpawnActorFromClass` Class (`KismetMathLibrary.MakeTransform` Location) "Undefined" "OverrideRootScale"))
  (`/Engine/EditorBlueprintResources/StandardMacros.IncrementInt` (`self.TileCount`)
    (:`  `
      (`Actor.K2_DestroyActor` (`|GetArrayItem` _activeactorarray))
      (`KismetArrayLibrary.Array_Remove` _activeactorarray)
      (`KismetArrayLibrary.Array_Add` _activeactorarray _returnvalue))))

(fn `SpawnTileAtStart`
  (params (TileActor :type "Actor Class Reference (by ref)"))
  (bind _returnvalue (`|SpawnActorFromClass` TileActor (`KismetMathLibrary.MakeTransform` (`KismetMathLibrary.MakeVector` (+ (.x (.location (`Actor.GetTransform` (`self.Character`)))) (* (`KismetMathLibrary.Conv_IntToDouble` (`self.TileSize`)) (`KismetMathLibrary.Conv_IntToDouble` (- (`self.TileCount`) 2)))) (+ (.y (.location (`Actor.GetTransform` (`self.Character`)))) (`self.TileY`)) (.z (.location (`Actor.GetTransform` (`self.Character`))))) (.rotation (`Actor.GetTransform` (`self.Character`))) (.scale (`Actor.GetTransform` (`self.Character`)))) "Undefined" "OverrideRootScale"))
  (`KismetArrayLibrary.Array_Add` (`self.ActiveActorArray`) _returnvalue))