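; BP_Rake is a clickable rake obstacle that arms a decelerator trap for a character when it falls.
; It starts with the upright broom mesh visible and its child BP_Decelerator collision off; clicking swaps to the ground mesh and enables query collision.
; When the decelerator reports a valid character, the rake disables that collision and switches the character's animation state for one second before setting another.
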(event `self.ReceiveBeginPlay`
  (bind _decelerator (`self.Decelerator`))
  (`SceneComponent.SetVisibility` (`self.BID_Broom_v01`) true false)
  (`SceneComponent.SetVisibility` (`self.Broom_ground`) false false)
  (bind _asbp_decelerator (cast `/Game/Core/Gameplay/BP_Decelerator` (`ChildActorComponent.ChildActor` (`self.BP_Decelerator`))))
  (set `self.Decelerator` _asbp_decelerator)
  (`PrimitiveComponent.SetCollisionEnabled` (`/Game/Core/Gameplay/BP_CharacterCollider.Box` _decelerator) "NoCollision")
  (add `/Game/Core/Gameplay/BP_CharacterCollider.onValidChar` _decelerator (delegate `receiveCharCollision`)))

(event `self.clicked`
  (`SceneComponent.SetVisibility` (`self.BID_Broom_v01`) false false)
  (`SceneComponent.SetVisibility` (`self.Broom_ground`) true false)
  (`PrimitiveComponent.SetCollisionEnabled` (`/Game/Core/Gameplay/BP_CharacterCollider.Box` (`self.Decelerator`)) "QueryOnly"))

(event `receiveCharCollision`
  (bind _animationhandler (`/Game/Core/Player/Blueprints/BP_Character.AnimationHandler` (`/Game/Core/Gameplay/BP_CharacterCollider.BP_Character` (`self.Decelerator`))))
  (`PrimitiveComponent.SetCollisionEnabled` (`/Game/Core/Gameplay/BP_CharacterCollider.Box` (`self.Decelerator`)) "NoCollision")
  (`/Game/Core/Animation/AnimationHandler.setAnimation` _animationhandler "NewEnumerator2")
  (`KismetSystemLibrary.Delay` 1.0)
  (`/Game/Core/Animation/AnimationHandler.setAnimation` _animationhandler "NewEnumerator1"))

(fn `UserConstructionScript`)