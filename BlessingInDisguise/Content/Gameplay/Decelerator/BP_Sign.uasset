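; Clickable sign actor that drops under physics and arms a decelerator collider when clicked.
; On BeginPlay it gets the BP_CharacterCollider from its BPDecelerator child actor, disables that sphere's collision and binds to its valid-character event.
; A click enables physics on the sign mesh and query-only collision on the sphere.
; When the collider reports a valid character, the sphere is disabled again and the event rebound.
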(event `self.ReceiveBeginPlay`
  (bind _asbp_character_collider (cast `/Game/Core/Gameplay/BP_CharacterCollider` (`ChildActorComponent.ChildActor` (`self.BP_Decelerator`))))
  (`PrimitiveComponent.SetCollisionEnabled` (`/Game/Core/Gameplay/BP_CharacterCollider.Sphere` _asbp_character_collider) "NoCollision" :!label _label)
  (add `/Game/Core/Gameplay/BP_CharacterCollider.onValicChar` _asbp_character_collider (delegate `CustomEvent_0`)))

(event `self.clicked`
  (`PrimitiveComponent.SetSimulatePhysics` (`self.sign_00`) true)
  (`PrimitiveComponent.SetCollisionEnabled` (`/Game/Core/Gameplay/BP_CharacterCollider.Sphere` (stale `self.ReceiveBeginPlay` _asbp_character_collider)) "QueryOnly"))

(event `CustomEvent_0`
  (goto _label))

(fn `UserConstructionScript`)